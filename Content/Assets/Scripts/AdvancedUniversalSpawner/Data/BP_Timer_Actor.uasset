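; BP_Timer_Actor is a helper actor for the Advanced Universal Spawner that schedules respawns for one spawner entry by Id.
; Once started, it loops a named-function timer with a random delay in the configured range, calling back to the spawner to respawn each time.
; The loop pauses when the spawner's max-count check fails and ends permanently when the respawn-limit check fails.
; Wave modes, or Main Spawn with respawn disabled, mark it ended at BeginPlay.
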(event EventBeginPlay
  (switch Utilities|FlowControl|Switch|SwitchonE_SpawnerModes (Variables|/Game/Assets/Scripts/AdvancedUniversalSpawner/Blueprints/BP_SplineSpawner.BP_SplineSpawner_C|GetSpawnerMode (Variables|Default|GetSpawnerRef))
    (:NewEnumerator0
      (if (not (.Respawn (Utilities|Struct|BreakStr_RespawnSettings (.RespawnSettings (Utilities|Struct|BreakStr_Respawn_Types (Variables|Default|GetRespawnInfo))))))
        (Variables|Default|SetRespawnEnd true :!label _label)))
    (:NewEnumerator1
      (goto _label))
    (:NewEnumerator2
      (goto _label))))

(fn ConstructionScript)

(fn -UpdateTimer
  (bind _id (Variables|Default|GetId))
  (bind _respawninfo (Variables|Default|GetRespawnInfo))
  (bind _spawnerref (Variables|Default|GetSpawnerRef))
  (bind _respawnsettings (Utilities|Struct|BreakStr_Respawn_Types _respawninfo))
  (bind (_timetorespawnmin _timetorespawnmax) (Utilities|Struct|BreakStr_RespawnSettings _respawnsettings))
  (if (Default|-CheckMaxCount _spawnerref _id)
    (if (Default|-CheckRespawnLimit _spawnerref _id)
      (bind _returnvalue (Utilities|Time|SetTimerbyFunctionName 0 "-Timer" (Math|Random|RandomFloatinRange _timetorespawnmin _timetorespawnmax)))
      (Variables|Default|SetTimer-Timer _returnvalue)
      (else
        (Variables|Default|SetRespawnEnd true)
        (Variables|Default|SetRespawnLaunched false)))
    (else
      (Variables|Default|SetRespawnLaunched false))))

(fn -Timer
  (Default|-CalltoRespawn (Variables|Default|GetSpawnerRef) (Variables|Default|GetId))
  (CallFunction|-UpdateTimer))

(fn -CalltoStartRespawnTimer
  (if (and (not (Variables|Default|GetRespawnLaunched)) (not (Variables|Default|GetRespawnEnd)))
    (Variables|Default|SetRespawnLaunched true)
    (CallFunction|-UpdateTimer)))