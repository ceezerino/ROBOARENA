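; BPC_UITrigger is a Blueprint component that triggers the end-of-game victory and defeat screens.
; SpawnVictoryUI and SpawnDefeatUI each cast the first player controller to BP_VERGEPlayerControler, switch it to UI mode, call its Victory or Defeated function, then pause the game.
; The screens are left to the controller, and a failed cast skips both the UI calls and the pause.
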(event Custom|Spawn%20Defeat%20UI
  (bind _asbp_vergeplayer_controler (Utilities|Casting|CastToBP_VERGEPlayerControler (Game|GetPlayerController 0)))
  (Default|UIMode _asbp_vergeplayer_controler)
  (Default|Defeated _asbp_vergeplayer_controler)
  (Game|SetGamePaused true))

(event Custom|Spawn%20Victory%20UI
  (bind _asbp_vergeplayer_controler (Utilities|Casting|CastToBP_VERGEPlayerControler (Game|GetPlayerController 0)))
  (Default|UIMode _asbp_vergeplayer_controler)
  (Default|Victory _asbp_vergeplayer_controler)
  (Game|SetGamePaused true))

(event EventBeginPlay)

(event EventTick
  (params (DeltaSeconds :type Float%20%28single-precision%29)))