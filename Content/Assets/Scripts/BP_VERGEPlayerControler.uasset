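; VERGE player controller that handles input mode switching and the victory and defeat screens.
; It caches BP_PlayerHUD on BeginPlay and toggles the mouse cursor between UI and game input modes.
; Victory and Defeated reveal their HUD widgets, with Defeated also playing a death sound and stopping the FullHealth sound.
; The logic that would spawn that vital sound is disconnected and never runs.
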(event Custom|UI%20Mode
  (Input|SetInputModeGameandUI (Game|GetPlayerController 0) 0 "DoNotLock" false false)
  (Variables|Default|SetbShowMouseCursor true))

(event Custom|Game%20Mode
  (Input|SetInputModeGameOnly (Game|GetPlayerController 0) false)
  (Variables|Default|SetbShowMouseCursor false))

(event Custom|Defeated
  (Widget|SetVisibility (Variables|/Game/Assets/UI/BP_PlayerHUD.BP_PlayerHUD_C|GetWB_DefeatedWidget (Variables|Default|GetBP%20Player%20HUD)) "Visible")
  ;[0.15 0.15 0.15 0.5] Death
  (Audio|SpawnSound2D "/Game/Sound/Player_Character/Vitals/PC_V_Death_Cue.PC_V_Death_Cue" 1.0 1.0 0.0 0)
  ;[0.15 0.15 0.15 0.5] Stop Vital Sounds
  (Audio|Components|Audio|Stop (Variables|Default|GetFullHealth)))

(event Custom|Victory
  (Widget|SetVisibility (Variables|/Game/Assets/UI/BP_PlayerHUD.BP_PlayerHUD_C|GetWB_Victory (Variables|Default|GetBP%20Player%20HUD)) "Visible"))

(event EventBeginPlay
  (bind _asbp_player_hud (Utilities|Casting|CastToBP_PlayerHUD (HUD|GetHUD)))
  (Variables|Default|SetBP%20Player%20HUD _asbp_player_hud))

(event EventTick
  (params (DeltaSeconds :type Float%20%28single-precision%29)))

(fn ConstructionScript)