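; Flying ranged enemy that hunts the player once detected and fires bullets when within ideal range.
; A looping timer switches homing projectile movement between a randomly repositioned invisible waypoint and the player, chasing the player after the waypoint is reached.
; In range, it halts, rotates toward the player via timed interpolation and shoots on a cooldown.
; If the player has left after enough shots, it stops aiming and heads for the waypoint again.
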(event OnComponentBeginOverlap(DetectionRadius)
  (params (OverlappedComponent :type Primitive%20Component%20Object%20Reference) (OtherActor :type Actor%20Object%20Reference) (OtherComp :type Primitive%20Component%20Object%20Reference) (OtherBodyIndex :type Integer) (bFromSweep :type Boolean) (SweepResult :type Hit%20Result%20Structure%20%28by%20ref%29))
  ;[0.15 0.15 0.15 0.5] Radius Logic
  (if (== OtherActor (Variables|Default|GetAs%20Player%20BP))
    (Utilities|FlowControl|DoOnce false
      (:Completed
        (Utilities|Time|SetTimerbyFunctionName 0 "Move Choice" 0.1 true true)))))

(event OnComponentBeginOverlap(IdealRange)
  (params (OverlappedComponent :type Primitive%20Component%20Object%20Reference) (OtherActor :type Actor%20Object%20Reference) (OtherComp :type Primitive%20Component%20Object%20Reference) (OtherBodyIndex :type Integer) (bFromSweep :type Boolean) (SweepResult :type Hit%20Result%20Structure%20%28by%20ref%29))
  ;[0.15 0.15 0.15 0.5] Radius Logic
  (if (== OtherActor (Variables|Default|GetAs%20Player%20BP))
    (Variables|Default|SetIn%20Ideal%20Range true)
    (Utilities|Time|SetTimerbyFunctionName 0 "Look!" 0.01 true)
    (elif (== OtherActor (Variables|Default|GetMovement%20Point))
      (Variables|Default|SetReached%20Movement%20Point true)
      (CallFunction|ResetPlayerChase)
      (CallFunction|ResetMovementPointChase))))

(event OnComponentEndOverlap(IdealRange)
  (params (OverlappedComponent :type Primitive%20Component%20Object%20Reference) (OtherActor :type Actor%20Object%20Reference) (OtherComp :type Primitive%20Component%20Object%20Reference) (OtherBodyIndex :type Integer))
  ;[0.15 0.15 0.15 0.5] Radius Logic
  (if (== OtherActor (Variables|Default|GetAs%20Player%20BP))
    (Variables|Default|SetIn%20Ideal%20Range false)
    (CallFunction|ResetPlayerChase)
    (CallFunction|ResetMovementPointChase)))

(event Custom|Begin%20Chase
  (params (Chase%20Target :type Scene%20Component%20Object%20Reference))
  (bind _flyingmovment (Variables|Default|GetFlyingMovment))
  ;[0.15 0.15 0.15 0.5] Core Movement
  ;;[0.15 0.15 0.15 0.5] Chase
  (Variables|/Script/Engine.ProjectileMovementComponent|SetHomingAccelerationMagnitude _flyingmovment 1e+03)
  (Variables|/Script/Engine.ProjectileMovementComponent|SetInitialSpeed _flyingmovment 7e+02)
  (Variables|/Script/Engine.ProjectileMovementComponent|SetHomingTargetComponent (Variables|Default|GetFlyingMovment) Chase%20Target))

(event Custom|Spawn%20Target%20Location
  ;[0.15 0.15 0.15 0.5] Relocate Functions
  ;;[0.15 0.15 0.15 0.5] Spawn Movement Point
  (bind _returnvalue (Game|SpawnActorfromClass "/Game/Assets/Enemies/BP_InvisibleTarget.BP_InvisibleTarget_C" (Math|Transform|MakeTransform "0, 0, 0" "0, 0, 0" "1.000000,1.000000,1.000000") "Undefined" "MultiplyWithRoot" 0 0))
  (Variables|Default|SetMovement%20Point _returnvalue)
  (CallFunction|MovemTargetedPoint))

(event Custom|Reset%20Movement%20Point%20Chase
  ;[0.15 0.15 0.15 0.5] Core Movement
  ;;[0.15 0.15 0.15 0.5] Choice Branching
  (Utilities|FlowControl|DoOnce false) ; enters at Reset
)

(event Custom|Reset%20Player%20Chase
  ;[0.15 0.15 0.15 0.5] Core Movement
  ;;[0.15 0.15 0.15 0.5] Choice Branching
  (Utilities|FlowControl|DoOnce false) ; enters at Reset
)

(event Custom|Shoot
  (bind _staticmesh (Variables|Default|GetStaticMesh))
  (bind _returnvalue (Transformation|GetWorldLocation _staticmesh))
  ;[0.15 0.15 0.15 0.5] Core Movement
  ;;[0.15 0.15 0.15 0.5] Shoot
  (Audio|PlaySoundatLocation "/Game/Sound/Enemys/MS_RangedAttack.MS_RangedAttack" (Transformation|GetActorLocation) "0, 0, 0" 1.0 1.0 0.0 0 0 0 0)
  (bind _returnvalue_2 (Game|SpawnActorfromClass "/Game/Assets/Enemies/BP_Bullet.BP_Bullet_C" (Math|Transform|MakeTransform (Math|Vector|MakeVector (.x _returnvalue) (.y _returnvalue) (.z _returnvalue)) "0, 0, 0" "1.000000,1.000000,1.000000") "AdjustIfPossibleButAlwaysSpawn" "MultiplyWithRoot" 0 0))
  (Physics|AddImpulse (Variables|/Game/Assets/Enemies/BP_Bullet.BP_Bullet_C|GetSphere _returnvalue_2) (* (- (Transformation|GetActorLocation (Variables|Default|GetAs%20Player%20BP)) (Transformation|GetWorldLocation _staticmesh)) (Variables|Default|GetProjectileSpeed)) "None" true)
  (CallFunction|MovemTargetedPoint))

(event Custom|Movem%20Targeted%20Point
  (bind _returnvalue (Math|Random|RandomFloatinRange -2.5e+03 2.5e+03))
  (bind _returnvalue_2 (Math|Vector|VectorZero))
  ;[0.15 0.15 0.15 0.5] Relocate Functions
  ;;[0.15 0.15 0.15 0.5] Move Targeted Point
  (Transformation|SetActorLocation (Variables|Default|GetMovement%20Point) (Math|Vector|MakeVector (+ _returnvalue (.x _returnvalue_2)) (+ _returnvalue (.y _returnvalue_2)) (+ (Math|Random|RandomFloatinRange 1.2e+03 1.85e+03) (.z _returnvalue_2))) true false))

(event Custom|Stay%20Put
  (bind _flyingmovment (Variables|Default|GetFlyingMovment))
  ;[0.15 0.15 0.15 0.5] Core Movement
  ;;[0.15 0.15 0.15 0.5] Stay Put
  (Variables|/Script/Engine.ProjectileMovementComponent|SetHomingAccelerationMagnitude _flyingmovment 0.0)
  (Game|Components|ProjectileMovement|SetVelocityinLocalSpace _flyingmovment "0, 0, 0")
  (Utilities|FlowControl|DoOnce false :!label _label
    (:Completed
      (CallFunction|Shoot)
      (Math|Integer|IncrementInt (Variables|Default|GetShot#)
        (:%20%20
          (Utilities|FlowControl|Delay (Variables|Default|GetShot%20Cooldown))
          (if (Variables|Default|GetIn%20Ideal%20Range)
            (CallFunction|StayPut)
            (goto _label Reset)
            (else
              (CallFunction|MovemTargetedPoint)
              (CallFunction|CheckRelocation)
              (Utilities|Time|SetTimerbyFunctionName 0 "Move Choice" 0.1 true)
              (goto _label Reset))))))))

(event Custom|Look!
  ;[0.15 0.15 0.15 0.5] Core Movement
  ;;[0.15 0.15 0.15 0.5] Aim at Player
  (Transformation|SetActorRotation (Math|Interpolation|RInterpTo (Transformation|GetActorRotation) (Math|Rotator|FindLookatRotation (Transformation|GetActorLocation) (Transformation|GetActorLocation (Game|GetPlayerCharacter 0))) 0.01 15.0)))

(event Custom|Move%20Choice
  ;[0.15 0.15 0.15 0.5] Core Movement
  ;;[0.15 0.15 0.15 0.5] Choice Branching
  (if (Variables|Default|GetIn%20Ideal%20Range)
    (CallFunction|StayPut)
    (elif (Variables|Default|GetReached%20Movement%20Point)
      (Utilities|FlowControl|DoOnce false
        (:Completed
          (CallFunction|BeginChase (Variables|/Script/Engine.Character|GetMesh (Variables|Default|GetAs%20Player%20BP)))))
      (else
        (Utilities|FlowControl|DoOnce false
          (:Completed
            (CallFunction|BeginChase (Variables|/Script/Engine.Actor|GetRootComponent (Variables|Default|GetMovement%20Point)))))))))

(event Custom|Check%20Relocation
  ;[0.15 0.15 0.15 0.5] Relocate Functions
  ;;[0.15 0.15 0.15 0.5] Relocation
  (if (>= (Variables|Default|GetShot#) 2)
    (Variables|Default|SetShot# 0)
    (Variables|Default|SetReached%20Movement%20Point false)
    (Utilities|Time|SetTimerbyFunctionName 0 "Look!" -1.0 true)))

(event EventBeginPlay
  ;[0.15 0.15 0.15 0.5] Startup
  (bind _asplayer_bp (Utilities|Casting|CastToPlayerBP (Game|GetPlayerCharacter 0)))
  (Variables|Default|SetAs%20Player%20BP _asplayer_bp)
  (CallFunction|SpawnTargetLocation))

(event Collision|EventActorBeginOverlap
  (params (OtherActor :type Actor%20Object%20Reference))
  ;[0.15 0.15 0.15 0.5] Radius Logic
)

(event EventTick
  (params (DeltaSeconds :type Float%20%28single-precision%29)))

(fn ConstructionScript)