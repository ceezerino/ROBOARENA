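; Projectile Blueprint, apparently for flying enemies, that damages the player on impact.
; The sphere's hit event checks the other actor: a PlayerBP hit applies fixed damage to player pawn 0, while BP_FlyingEnemy hits are ignored.
; Player and all other hits spawn a scaled-up magic impact effect oriented along the normal impulse, print its name, then destroy the bullet.
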(event OnComponentHit(Sphere)
  (params (HitComponent :type Primitive%20Component%20Object%20Reference) (OtherActor :type Actor%20Object%20Reference) (OtherComp :type Primitive%20Component%20Object%20Reference) (NormalImpulse :type Vector :default "0, 0, 0") (Hit :type Hit%20Result%20Structure%20%28by%20ref%29))
  (Class|KismetSystemLibrary|IsObjectOfSoftClass OtherActor "/Game/Assets/Scripts/Player/PlayerBP.PlayerBP_C"
    (:True
      (Game|Damage|ApplyDamage (Game|Player|GetPlayerPawn 0) 1e+01 0 0))
    (:False
      (Class|KismetSystemLibrary|IsObjectOfSoftClass OtherActor "/Game/Assets/Enemies/Flying/BP_FlyingEnemy.BP_FlyingEnemy_C"
        (:False
          _))))
  (bind _returnvalue (Niagara|SpawnSystematLocation "/Game/Assets/VFX/ImpactEffects/Realistic_Starter_VFX_Pack_Vol2/Particles/Hit/P_MagicImpact.P_MagicImpact" (Transformation|GetWorldLocation (Variables|Default|GetSphere)) (Math|Conversions|RotationFromXVector NormalImpulse) "7.000000,7.000000,7.000000"))
  (Development|PrintString (Utilities|GetDisplayName _returnvalue))
  (Actor|DestroyActor))

(event EventBeginPlay)

(event Collision|EventActorBeginOverlap
  (params (OtherActor :type Actor%20Object%20Reference)))

(event EventTick
  (params (DeltaSeconds :type Float%20%28single-precision%29)))

(fn ConstructionScript)