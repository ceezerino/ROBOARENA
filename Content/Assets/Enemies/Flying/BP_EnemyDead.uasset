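; Debris actor for dead enemies that shows randomly chosen broken body meshes in gold material.
; DeathSpawn uses its Land flag to pick mesh sets: three scaled-up pieces for shield enemies, two for flying foes.
; It then calls DeathDisplay for audio, delayed Niagara effects and a timed lifespan, and fires a radial impulse to scatter the pieces.
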(event Custom|Death%20Spawn
  (params (Land? :type Boolean))
  (bind _staticmesh_1 (Variables|Default|GetStaticMesh_1))
  (bind _staticmesh_2 (Variables|Default|GetStaticMesh_2))
  (bind _static_mesh_3 (Variables|Default|GetStatic_Mesh_3))
  (if Land?
    ;[0.15 0.15 0.15 0.5] Random Body Meshes Whenever Shield Guys Die
    (Components|StaticMesh|SetStaticMesh _staticmesh_1 (Utilities|Array|Get(acopy) (Variables|Default|GetMeshPossibilities) (Math|Random|RandomIntegerinRange 4 6)))
    (Transformation|SetWorldScale3D _staticmesh_1 "1.100000,1.100000,1.100000")
    (Components|StaticMesh|SetStaticMesh _staticmesh_2 (Utilities|Array|Get(acopy) (Variables|Default|GetMeshPossibilities) (Math|Random|RandomIntegerinRange 7 9)))
    (Transformation|SetWorldScale3D _staticmesh_2 "1.100000,1.100000,1.100000")
    (Components|StaticMesh|SetStaticMesh _static_mesh_3 (Utilities|Array|Get(acopy) (Variables|Default|GetMeshPossibilities) (Math|Random|RandomIntegerinRange 4 6)))
    (Transformation|SetWorldScale3D _static_mesh_3 "1.100000,1.100000,1.100000")
    (Rendering|Material|SetMaterial _static_mesh_3 0 "/Game/Assets/CustomMaterials/Enemies/MI_EnemyGold.MI_EnemyGold")
    (else
      ;[0.15 0.15 0.15 0.5] Random Body Meshes Whenever Flying Foes Die
      (Components|StaticMesh|SetStaticMesh (Variables|Default|GetStaticMesh_1) (Utilities|Array|Get(acopy) (Variables|Default|GetMeshPossibilities) (Math|Random|RandomIntegerinRange 0 3)))
      (Components|StaticMesh|SetStaticMesh (Variables|Default|GetStaticMesh_2) (Utilities|Array|Get(acopy) (Variables|Default|GetMeshPossibilities) (Math|Random|RandomIntegerinRange 0 3)))))
  (Rendering|Material|SetMaterial (Variables|Default|GetStaticMesh_1) 0 "/Game/Assets/CustomMaterials/Enemies/MI_EnemyGold.MI_EnemyGold")
  (Rendering|Material|SetMaterial (Variables|Default|GetStaticMesh_2) 0 "/Game/Assets/CustomMaterials/Enemies/MI_EnemyGold.MI_EnemyGold")
  (CallFunction|DeathDisplay)
  (Class|RadialForceComponent|FireImpulse (Variables|Default|GetRadialForce))
  (Development|PrintString "FIRED"))

(event Custom|Death%20Display
  ;[0.15 0.15 0.15 0.5] How Broken Meshes Behave When Spawned
  (Actor|SetLifeSpan 1e+01)
  (Audio|Components|Audio|Play (Variables|Default|GetAudio) 0.0)
  (Utilities|FlowControl|Delay 0.2)
  (Components|Activation|Activate (Variables|Default|GetNiagara) false)
  (Components|Activation|Activate (Variables|Default|GetNiagara1) false))

(event EventTick
  (params (DeltaSeconds :type Float%20%28single-precision%29)))

(event EventBeginPlay)

(fn ConstructionScript)