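; Player character Blueprint for fast movement, with crouch slide, air slam, dash, wall slide and jump, and a grapple.
; Enhanced Input events drive launch impulses, gravity and friction changes, with sound and particle feedback.
; Tick regenerates dash stamina and, while airborne, traces left and right for walls, storing normals for wall jumps.
; Landing fires buffered jumps or slam effects; the grapple line-traces from the actor along camera forward and launches toward the hit.
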(event Custom|Detect%20Wall
  (bind _capsulecomponent (Variables|Collision|GetCapsuleComponent))
  (bind _charactermovement (Variables|Character|GetCharacterMovement))
  (bind _returnvalue (Transformation|GetWorldLocation _capsulecomponent))
  ;[0.15 0.15 0.15 0.5] Wall Jump Detection Logic
  (if (AI|Components|NavMovement|IsFalling (Variables|Character|GetCharacterMovement))
    (Utilities|FlowControl|Sequence
      (:then_0
        (if (Variables|Default|GetWallJump?)
          _
          (else
            (Variables|Default|SetRight? true)))
        (bind (_outhit _returnvalue_2) (Collision|LineTraceByChannel _returnvalue (+ _returnvalue (* (Math|Vector|GetRightVector _capsulecomponent) (Variables|Default|GetWallCheckDistance))) "TraceTypeQuery3" false 0 "None"))
        (Variables|Default|SetRightNormal (.impactnormal _outhit)))
      (:then_1
        (if (Variables|Default|GetWallJump?)
          _
          (else
            (Variables|Default|SetRight? false)))
        (bind (_outhit_2 _returnvalue_3) (Collision|LineTraceByChannel _returnvalue (+ _returnvalue (* (* (Math|Vector|GetRightVector _capsulecomponent) -1) (Variables|Default|GetWallCheckDistance))) "TraceTypeQuery1" false 0 "None"))
        (Variables|Default|SetLeftNormal (.impactnormal _outhit_2))))
    (if (or _returnvalue_2 _returnvalue_3)
      (Variables|Default|SetWallJump? true)
      (Variables|/Script/Engine.MovementComponent|SetVelocity _charactermovement (Math|Interpolation|VInterptoConstant (Variables|/Script/Engine.MovementComponent|GetVelocity _charactermovement) "0, 0, 0" (Utilities|Time|GetWorldDeltaSeconds) 0.0))
      (else
        (Variables|Default|SetWallJump? false :!label _label)))
    (else
      (goto _label))))

(event Custom|Stamina%20Regen
  ;[0.15 0.15 0.15 0.5] Stamina Regen
  (if (not (>= (Variables|Default|GetStamina) 2.0))
    (Variables|Default|SetStamina (+ (Variables|Default|GetStamina) 0.01))))

(event Custom|SlamVFX
  (bind _returnvalue (Game|GetPlayerCharacter 0))
  (bind _returnvalue_2 (Transformation|GetActorLocation _returnvalue))
  ;[0.15 0.15 0.15 0.5] Slam
  (Niagara|SpawnSystematLocation (Utilities|Array|Get(acopy) (Variables|Default|GetParticleArray) 1) _returnvalue_2 "0, 0, 0" "3.000000,3.000000,1.000000")
  (Audio|PlaySoundatLocation "/Game/Sound/Player_Character/Grapple/PCA_G_Charge.PCA_G_Charge" _returnvalue_2 "0, 0, 0" 1.0 1.0 0.0 0 0 0 0))

(event Custom|Slide
  (bind _charactermovement (Variables|Character|GetCharacterMovement))
  (bind _slideslowdown (Variables|Default|GetSlideSlowdown))
  ;[0.15 0.15 0.15 0.5] Sliding
  (Utilities|FlowControl|DoOnce false
    (:Completed
      (Audio|SpawnSoundAttached "/Game/Sound/Player_Character/Boost/PCA_B_Slide.PCA_B_Slide" (Variables|Character|GetMesh) "None" "0, 0, 0" "0, 0, 0" "KeepRelativeOffset" false 1.0 1.0 0.0 0 0)
      (if (not (Variables|Default|GetSlideLock))
        (if (>= (Math|Vector|VectorLength (* (Variables|/Script/Engine.MovementComponent|GetVelocity _charactermovement) "1.000000,1.000000,0.000000")) 6e+02)
          (if (Variables|Default|GetWallJump?)
            (if (Variables|Default|GetWallSlide?)
              (if (>= (Math|Vector|VectorLength (* (Variables|/Script/Engine.MovementComponent|GetVelocity _charactermovement) "1.000000,1.000000,0.000000")) 6e+02)
                (Variables|Default|SetWallSlide? false)
                (else
                  (Variables|Default|SetWallSlide? true)))
              (Variables|/Script/Engine.MovementComponent|SetVelocity _charactermovement (Math|Vector|MakeVector (* (.x (Variables|/Script/Engine.MovementComponent|GetVelocity _charactermovement)) _slideslowdown) (* (.y (Variables|/Script/Engine.MovementComponent|GetVelocity _charactermovement)) _slideslowdown) 0.0))
              (Variables|/Script/Engine.CharacterMovementComponent|SetGravityScale _charactermovement 0.4)
              (else
                (Variables|Default|SetWallSlide? false :!label _label)))
            (else
              (Variables|/Script/Engine.CharacterMovementComponent|SetGravityScale _charactermovement (Variables|Default|GetGravity))
              (goto _label)))
          (Character|Crouch)
          (else
            (CallFunction|SlideComplete)
            (Variables|Default|SetSlideLock true)))))))

(event Custom|Slide_Complete
  (bind _charactermovement (Variables|Character|GetCharacterMovement))
  (bind _slideslowdown (Variables|Default|GetSlideSlowdown))
  ;[0.15 0.15 0.15 0.5] Sliding
  (Variables|Default|SetSlideLock false)
  (Variables|Default|SetisSliding? false)
  (if (Variables|Default|GetWallSlide?)
    (Variables|/Script/Engine.CharacterMovementComponent|SetGravityScale _charactermovement (Variables|Default|GetGravity))
    (Variables|Default|SetWallSlide? false))
  (Character|UnCrouch)
  (Utilities|FlowControl|DoOnce false) ; enters at Reset
)

(event Custom|Slide_Start
  (bind _returnvalue (Class|Pawn|GetLastMovementInputVector))
  (bind _moving_ (Variables|Default|GetMoving?))
  (bind _capsulecomponent (Variables|Collision|GetCapsuleComponent))
  (bind _returnvalue_2 (Math|Vector|GetForwardVector _capsulecomponent))
  (bind _returnvalue_3 (Math|Vector|SelectVector _returnvalue _returnvalue_2 _moving_))
  ;[0.15 0.15 0.15 0.5] Sliding
  (Character|Crouch)
  (if (Variables|Default|GetWallJump?)
    (Variables|Default|SetWallSlide? true)
    (Character|LaunchCharacter (* _returnvalue_3 (Variables|Default|GetWallBoost)) false false)
    (else
      (Character|LaunchCharacter (* _returnvalue_3 (Variables|Default|GetSlideBoost)) false false))))

(event Custom|Slam
  ;[0.15 0.15 0.15 0.5] Slam
  (Variables|Default|SetSlammed? true)
  (Character|LaunchCharacter (Math|Vector|MakeVector 0.0 0.0 (Variables|Default|GetSlam%20Speed)) true true))

(event Custom|Slam_Release
  ;[0.15 0.15 0.15 0.5] Slam
  (Variables|Default|SetSlammed? false))

(event Custom|Grapple%20Fire
  ;[0.15 0.15 0.15 0.5] Grapple Fire
)

(event Custom|Reset%20Grapple
  ;[0.15 0.15 0.15 0.5] Reset Grapple
  (Rendering|SetVisibility (Variables|Default|GetGrapple) false false)
  (Variables|Default|SetGrapple? false)
  (Utilities|FlowControl|Delay 0.5))

(event Custom|Grapple%20Impact
  (params (GrappleEnd :type Vector) (GrappleOrigin :type Vector))
  (bind _returnvalue (Math|Rotator|FindLookatRotation GrappleEnd GrappleOrigin))
  ;[0.15 0.15 0.15 0.5] Grapple Particle
  (Audio|PlaySoundatLocation "/Game/Sound/Player_Character/Grapple/PCA_G_Attach.PCA_G_Attach" GrappleEnd "0, 0, 0" 1.0 1.0 0.0 0 0 0 0)
  (Niagara|SpawnSystematLocation (Utilities|Array|Get(acopy) (Variables|Default|GetParticleArray)) GrappleEnd (Math|Rotator|MakeRotator 0.0 (+ (.pitch _returnvalue) 9e+01) (.yaw _returnvalue)) "200.000000,200.000000,200.000000")
  (Audio|SpawnSoundatLocation 0 "0, 0, 0" "0, 0, 0" 1.0 1.0 0.0 0 0))

(event Input|EnhancedActionEvents|EnhancedInputActionIA_Move
  (params (ActionValue :type Vector%202D%20Structure) (ElapsedSeconds :type Float%20%28double-precision%29) (TriggeredSeconds :type Float%20%28double-precision%29) (InputAction :type Input%20Action%20Object%20Reference :default "/Game/Assets/Scripts/IA_Move.IA_Move"))
  (bind (_x _y) (Math|Vector2D|BreakVector2D ActionValue))
  ;[0.15 0.15 0.15 0.5] Basic Movement
  (:Triggered
    (Variables|Default|SetMoving? true)
    (Pawn|Input|AddMovementInput (Math|Vector|GetRightVector (Pawn|GetControlRotation :!class /Script/Engine.Pawn)) _x false)
    (Pawn|Input|AddMovementInput (Math|Vector|GetForwardVector (Math|Rotator|MakeRotator 0.0 0.0 (.yaw (Pawn|GetControlRotation :!class /Script/Engine.Pawn)))) _y false))
  (:Completed
    (Variables|Default|SetMoving? false)))

(event Input|EnhancedActionEvents|EnhancedInputActionIA_Look
  (params (ActionValue :type Vector%202D%20Structure) (ElapsedSeconds :type Float%20%28double-precision%29) (TriggeredSeconds :type Float%20%28double-precision%29) (InputAction :type Input%20Action%20Object%20Reference :default "/Game/Assets/Scripts/IA_Look.IA_Look"))
  ;[0.15 0.15 0.15 0.5] Camera Control
  (Pawn|Input|AddControllerYawInput (.x ActionValue))
  (Pawn|Input|AddControllerPitchInput (.y ActionValue)))

(event Input|EnhancedActionEvents|EnhancedInputActionIA_Jump
  (params (ActionValue :type Boolean) (ElapsedSeconds :type Float%20%28double-precision%29) (TriggeredSeconds :type Float%20%28double-precision%29) (InputAction :type Input%20Action%20Object%20Reference :default "/Game/Assets/Scripts/IA_Jump.IA_Jump"))
  (bind _charactermovement (Variables|Character|GetCharacterMovement))
  ;[0.15 0.15 0.15 0.5] Jump Logic
  (Audio|PlaySoundatLocation "/Game/Sound/Player_Character/Jump/PCA_J_Start.PCA_J_Start" (Transformation|GetWorldLocation (Variables|Collision|GetCapsuleComponent)) "0, 0, 0" 1.0 1.0 0.0 0 0 0 0)
  (if (Variables|Default|GetWallJump?)
    (if (Variables|Default|GetRight?)
      (Variables|Default|SetUsed%20Normal (Variables|Default|GetRightNormal))
      (else
        (Variables|Default|SetUsed%20Normal (Variables|Default|GetLeftNormal))))
    (Character|LaunchCharacter (Math|Vector|MakeVector (.x (* (Math|Vector|Normalize (+ (* (Math|Vector|GetForwardVector (Variables|Collision|GetCapsuleComponent)) 1.0) (* (Variables|Default|GetUsed%20Normal) 2.0))) (Variables|Default|GetWallJumpForce))) (.y (* (Math|Vector|Normalize (+ (* (Math|Vector|GetForwardVector (Variables|Collision|GetCapsuleComponent)) 1.0) (* (Variables|Default|GetUsed%20Normal) 2.0))) (Variables|Default|GetWallJumpForce))) (+ 0.0 1e+03)) false true)
    (elif (AI|Components|NavMovement|IsCrouching _charactermovement)
      (Character|UnCrouch)
      (Character|Jump :!label _label)
      (elif (Variables|Default|GetDashing?)
        (Character|LaunchCharacter (Math|Vector|MakeVector 0.0 0.0 1e+03) false false)
        (elif (AI|Components|NavMovement|IsFalling _charactermovement)
          (Variables|Default|SetJumpBuffered? true)
          (Utilities|FlowControl|Delay (Variables|Default|GetBufferTime))
          (Variables|Default|SetJumpBuffered? false)
          (else
            (goto _label)))))))

(event Input|EnhancedActionEvents|EnhancedInputActionIA_Dash
  (params (ActionValue :type Boolean) (ElapsedSeconds :type Float%20%28double-precision%29) (TriggeredSeconds :type Float%20%28double-precision%29) (InputAction :type Input%20Action%20Object%20Reference :default "/Game/Assets/Scripts/IA_Dash.IA_Dash"))
  (bind _charactermovement (Variables|Character|GetCharacterMovement))
  (bind _charactermovement_2 (Variables|Character|GetCharacterMovement))
  ;[0.15 0.15 0.15 0.5] Dash
  (if (not (<= (Variables|Default|GetStamina) 1.0))
    (Variables|Default|SetDashing? true)
    (Variables|Default|SetStamina (- (Variables|Default|GetStamina) 1.0))
    (Variables|/Script/Engine.CharacterMovementComponent|SetGravityScale _charactermovement 0.0)
    (if (Variables|Default|GetMoving?)
      (Character|LaunchCharacter (* (Class|Pawn|GetLastMovementInputVector) (Variables|Default|GetLaunchForce)) false false)
      (else
        (Character|LaunchCharacter (* (Math|Vector|Normalize (Math|Vector|GetForwardVector (Variables|Collision|GetCapsuleComponent))) (Variables|Default|GetLaunchForce)) false false)))
    (Audio|SpawnSoundAttached "/Game/Sound/Player_Character/Boost/PCA_B_Boost.PCA_B_Boost" (Variables|Collision|GetCapsuleComponent) "None" "0, 0, 0" "0, 0, 0" "KeepRelativeOffset" false 1.0 1.0 0.0 0 0)
    (Utilities|FlowControl|Delay 0.2)
    (Variables|/Script/Engine.CharacterMovementComponent|SetGravityScale _charactermovement (Variables|Default|GetGravity))
    (Variables|Default|SetDashing? false)
    (if (not (Variables|Default|GetisSliding?))
      (if (not (AI|Components|NavMovement|IsFalling _charactermovement_2))
        (Variables|/Script/Engine.MovementComponent|SetVelocity _charactermovement_2 "0, 0, 0")))))

(event Input|EnhancedActionEvents|EnhancedInputActionIA_Crouch
  (params (ActionValue :type Boolean) (ElapsedSeconds :type Float%20%28double-precision%29) (TriggeredSeconds :type Float%20%28double-precision%29) (InputAction :type Input%20Action%20Object%20Reference :default "/Game/Assets/Scripts/IA_Crouch.IA_Crouch"))
  ;[0.15 0.15 0.15 0.5] Crouch
  (:Triggered
    (if (not (Variables|Default|GetSlideLock))
      (CallFunction|Slide)))
  (:Started
    (if (Variables|Default|GetWallJump?)
      (Variables|Default|SetWallSlide? true)
      (CallFunction|Slide)
      (elif (AI|Components|NavMovement|IsFalling (Variables|Character|GetCharacterMovement))
        (CallFunction|Slam)
        (else
          (CallFunction|SlideStart)))))
  (:Completed
    (if (Variables|Default|GetSlammed?)
      (CallFunction|SlamRelease)
      (else
        (CallFunction|SlideComplete)))))

(event Input|EnhancedActionEvents|EnhancedInputActionIA_Grapple
  (params (ActionValue :type Boolean) (ElapsedSeconds :type Float%20%28double-precision%29) (TriggeredSeconds :type Float%20%28double-precision%29) (InputAction :type Input%20Action%20Object%20Reference :default "/Game/Assets/Scripts/IA_Grapple.IA_Grapple"))
  (bind _returnvalue (Transformation|GetActorLocation))
  (bind _camera (Variables|Default|GetCamera))
  (bind _grappledistance (Variables|Default|GetGrappleDistance))
  (bind _returnvalue_2 (Math|Vector|GetForwardVector _camera))
  (bind _returnvalue_3 (* _returnvalue_2 _grappledistance))
  (bind _returnvalue_4 (+ _returnvalue _returnvalue_3))
  ;[0.15 0.15 0.15 0.5] Main Grapple
  (:Started
    (if (Variables|Default|GetGrapple?)
      (CallFunction|ResetGrapple)
      (else
        (Audio|PlaySoundatLocation "/Game/Sound/Player_Character/Grapple/PCA_G_Out.PCA_G_Out" _returnvalue "0, 0, 0" 1.0 1.0 0.0 0 0 0 0)
        (bind (_outhit _returnvalue_5) (Collision|LineTraceByChannel _returnvalue _returnvalue_4 "TraceTypeQuery1" false 0 "None"))
        (if _returnvalue_5
          (bind _output_get (Variables|Default|SetGrapplePoint (.location _outhit)))
          (CallFunction|GrappleImpact _output_get _returnvalue_4)
          (Variables|Default|SetGrapple? true)
          (CallFunction|GrappleFire)
          (Character|LaunchCharacter "0.000000,0.000000,500.000000" true true)
          (Utilities|FlowControl|Delay 0.0)
          (Character|LaunchCharacter (* (- (Variables|Default|GetGrapplePoint) (Transformation|GetActorLocation)) 2.0) false false)
          (Utilities|FlowControl|Delay 0.4)
          (if (Variables|Default|GetGrapple?)
            (CallFunction|ResetGrapple))
          (else
            (CallFunction|ResetGrapple)))))))

(event EventBeginPlay
  ;[0.15 0.15 0.15 0.5] Player Start
  (Input|AddMappingContext (PlayerController|LocalPlayerSubsystems|GetEnhancedInputLocalPlayerSubsystem (Game|GetPlayerController 0)) "/Game/Assets/Scripts/IMC_Move.IMC_Move" 0 "(bIgnoreAllPressedKeysUntilRelease=True,bForceImmediately=False,bNotifyUserSettings=False)")
  (Variables|Default|SetGravity 3.0))

(event Collision|EventActorBeginOverlap
  (params (OtherActor :type Actor%20Object%20Reference)))

(event EventTick
  (params (DeltaSeconds :type Float%20%28single-precision%29))
  (Utilities|FlowControl|Sequence
    (:then_0
      (Variables|Default|SetDelta%20Seconds DeltaSeconds))
    (:then_1
      (CallFunction|StaminaRegen)
      (if (AI|Components|NavMovement|IsFalling (Variables|Character|GetCharacterMovement))
        (CallFunction|DetectWall)))))

(event EventOnLanded
  (params (Hit :type Hit%20Result%20Structure%20%28by%20ref%29))
  (bind _charactermovement (Variables|Character|GetCharacterMovement))
  ;[0.15 0.15 0.15 0.5] On Landed
  (Variables|Default|SetWallSlide? false)
  (Variables|Default|SetWallJump? false)
  (if (Variables|Default|GetJumpBuffered?)
    (Character|Jump)
    (elif (Variables|Default|GetSlammed?)
      (CallFunction|SlamRelease)
      (CallFunction|SlamVFX)
      (else
        (Variables|/Script/Engine.CharacterMovementComponent|SetGroundFriction _charactermovement 6.0)
        (Utilities|FlowControl|Delay 0.1)
        (Variables|/Script/Engine.CharacterMovementComponent|SetGroundFriction _charactermovement 2.0)))))

(fn ConstructionScript)

(fn CanJumpInternal
  (return (not (AI|Components|NavMovement|IsFalling (Variables|Character|GetCharacterMovement)))))