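; BP_FlyingEnemyDead is the remains actor for a dead flying enemy, a short-lived visual and audio death effect.
; On BeginPlay it gives two static mesh components random meshes from MeshPossibilities and applies the gold enemy material to both.
; It sets a lifespan so it destroys itself, plays its audio at once and activates the Niagara effect after a brief delay.
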(event EventTick
  (params (DeltaSeconds :type Float%20%28single-precision%29)))

(event EventBeginPlay
  (Components|StaticMesh|SetStaticMesh (Variables|Default|GetStaticMesh_1) (.OutItem (Utilities|Array|Random (Variables|Default|GetMeshPossibilities))))
  (Components|StaticMesh|SetStaticMesh (Variables|Default|GetStaticMesh_2) (.OutItem (Utilities|Array|Random (Variables|Default|GetMeshPossibilities))))
  (Rendering|Material|SetMaterial (Variables|Default|GetStaticMesh_1) 0 "/Game/Assets/CustomMaterials/Enemies/MI_EnemyGold.MI_EnemyGold")
  (Rendering|Material|SetMaterial (Variables|Default|GetStaticMesh_2) 0 "/Game/Assets/CustomMaterials/Enemies/MI_EnemyGold.MI_EnemyGold")
  (Actor|SetLifeSpan 1e+01)
  (Audio|Components|Audio|Play (Variables|Default|GetAudio) 0.0)
  (Utilities|FlowControl|Delay 0.2)
  (Components|Activation|Activate (Variables|Default|GetNiagara) false))

(fn ConstructionScript)