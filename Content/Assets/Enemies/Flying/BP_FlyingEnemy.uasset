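; Flying ranged enemy that faces the player, fires bullets and is replaced by a death actor on any damage.
; Homing movement, re-evaluated by a timer, chases a randomly placed invisible waypoint, then the player once that waypoint is reached.
; With the player inside IdealRange it halts and shoots on a cooldown, moving the waypoint after each shot.
; Overlapping another flyer briefly suspends that timer and homes it back to the waypoint.
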(event OnComponentBeginOverlap(Hitbox)
  (params (OverlappedComponent :type Primitive%20Component%20Object%20Reference) (OtherActor :type Actor%20Object%20Reference) (OtherComp :type Primitive%20Component%20Object%20Reference) (OtherBodyIndex :type Integer) (bFromSweep :type Boolean) (SweepResult :type Hit%20Result%20Structure%20%28by%20ref%29))
  ;[0.15 0.15 0.15 0.5] Radius Logic
  (Class|KismetSystemLibrary|IsObjectOfSoftClass OtherActor "/Game/Assets/Enemies/Flying/BP_FlyingEnemy.BP_FlyingEnemy_C"
    (:True
      (Utilities|Time|SetTimerbyFunctionName 0 "Move Choice" -1.0 true true)
      (CallFunction|BeginChase (Variables|/Script/Engine.Actor|GetRootComponent (Variables|Default|GetMovement%20Point)))
      (Utilities|FlowControl|Delay 0.25)
      (Utilities|Time|SetTimerbyFunctionName 0 "Move Choice" 0.1 true true))))

(event OnComponentBeginOverlap(IdealRange)
  (params (OverlappedComponent :type Primitive%20Component%20Object%20Reference) (OtherActor :type Actor%20Object%20Reference) (OtherComp :type Primitive%20Component%20Object%20Reference) (OtherBodyIndex :type Integer) (bFromSweep :type Boolean) (SweepResult :type Hit%20Result%20Structure%20%28by%20ref%29))
  ;[0.15 0.15 0.15 0.5] Radius Logic
  (if (== OtherActor (Variables|Default|GetMovement%20Point))
    (Variables|Default|SetReached%20Movement%20Point true)))

(event Custom|Begin%20Chase
  (params (Chase%20Target :type Scene%20Component%20Object%20Reference))
  (bind _flyingmovment (Variables|Default|GetFlyingMovment))
  (bind _flyingmovment_2 (Variables|Default|GetFlyingMovment))
  ;[0.15 0.15 0.15 0.5] Core Movement
  ;;[0.15 0.15 0.15 0.5] Chase
  (Variables|/Script/Engine.ProjectileMovementComponent|SetHomingAccelerationMagnitude _flyingmovment_2 (Variables|Default|GetAccel/Tunring))
  (Variables|/Script/Engine.ProjectileMovementComponent|SetInitialSpeed _flyingmovment_2 6e+02)
  (Variables|/Script/Engine.ProjectileMovementComponent|SetMaxSpeed _flyingmovment 1.4e+03)
  (Variables|/Script/Engine.ProjectileMovementComponent|SetHomingTargetComponent _flyingmovment Chase%20Target))

(event Custom|Spawn%20Target%20Location
  ;[0.15 0.15 0.15 0.5] Relocate Functions
  ;;[0.15 0.15 0.15 0.5] Spawn Movement Point
  (bind _returnvalue (Game|SpawnActorfromClass "/Game/Assets/Enemies/Flying/BP_InvisibleTarget.BP_InvisibleTarget_C" (Math|Transform|MakeTransform "0, 0, 0" "0, 0, 0" "1.000000,1.000000,1.000000") "Undefined" "MultiplyWithRoot" 0 0))
  (Variables|Default|SetMovement%20Point _returnvalue)
  (CallFunction|MovemTargetedPoint))

(event Custom|Shoot
  (bind _staticmesh (Variables|Default|GetStaticMesh))
  (bind _returnvalue (Transformation|GetWorldLocation _staticmesh))
  ;[0.15 0.15 0.15 0.5] Core Movement
  ;;[0.15 0.15 0.15 0.5] Shoot
  (Audio|PlaySoundatLocation "/Game/Sound/Enemys/MS_RangedAttack.MS_RangedAttack" (Transformation|GetActorLocation) "0, 0, 0" 1.0 1.0 0.0 0 0 0 0)
  (bind _returnvalue_2 (Game|SpawnActorfromClass "/Game/Assets/Enemies/Flying/BP_Bullet.BP_Bullet_C" (Math|Transform|MakeTransform (Math|Vector|MakeVector (.x _returnvalue) (.y _returnvalue) (.z _returnvalue)) "0, 0, 0" "1.000000,1.000000,1.000000") "AdjustIfPossibleButAlwaysSpawn" "MultiplyWithRoot" 0 0))
  (Physics|AddImpulse (Variables|/Game/Assets/Enemies/Flying/BP_Bullet.BP_Bullet_C|GetSphere _returnvalue_2) (* (- (Transformation|GetActorLocation (Variables|Default|GetAs%20Player%20BP)) (Transformation|GetWorldLocation _staticmesh)) (Variables|Default|GetProjectileSpeed)) "None" true)
  (CallFunction|MovemTargetedPoint))

(event Custom|Movem%20Targeted%20Point
  (bind _returnvalue (Math|Random|RandomFloatinRange -2.5e+03 2.5e+03))
  (bind _returnvalue_2 (Math|Vector|VectorZero))
  (bind _ideal_range (Variables|Default|GetIdeal%20Range))
  ;[0.15 0.15 0.15 0.5] Relocate Functions
  ;;[0.15 0.15 0.15 0.5] Move Targeted Point
  (Transformation|SetActorLocation (Variables|Default|GetMovement%20Point) (Math|Vector|MakeVector (+ _returnvalue (.x _returnvalue_2)) (+ _returnvalue (.y _returnvalue_2)) (+ (Math|Random|RandomFloatinRange 1.2e+03 1.85e+03) (.z _returnvalue_2))) true false)
  (if true
    (bind _returnvalue_3 (Class|PrimitiveComponent|SphereOverlapComponent (Variables|/Game/Assets/Enemies/Flying/BP_InvisibleTarget.BP_InvisibleTarget_C|GetCube (Variables|Default|GetMovement%20Point)) (Transformation|GetWorldLocation _ideal_range) (Components|Sphere|GetScaledSphereRadius _ideal_range) false false false))
    (if _returnvalue_3
      (CallFunction|MovemTargetedPoint))))

(event Custom|Stay%20Put
  (bind _flyingmovment (Variables|Default|GetFlyingMovment))
  ;[0.15 0.15 0.15 0.5] Core Movement
  ;;[0.15 0.15 0.15 0.5] Stay Put
  (Variables|/Script/Engine.ProjectileMovementComponent|SetHomingAccelerationMagnitude _flyingmovment 0.0)
  (Game|Components|ProjectileMovement|SetVelocityinLocalSpace _flyingmovment "0, 0, 0")
  (Utilities|FlowControl|DoOnce false :!label _label
    (:Completed
      (CallFunction|Shoot)
      (Math|Integer|IncrementInt (Variables|Default|GetShot#)
        (:%20%20
          (Utilities|FlowControl|Delay (Variables|Default|GetShot%20Cooldown))
          (if (stale Custom|Move%20Choice _still_in_range)
            (CallFunction|StayPut)
            (goto _label Reset)
            (else
              (CallFunction|MovemTargetedPoint)
              (CallFunction|CheckRelocation)
              (Utilities|Time|SetTimerbyFunctionName 0 "Move Choice" 0.1 true)
              (goto _label Reset))))))))

(event Custom|Look!
  ;[0.15 0.15 0.15 0.5] Core Movement
  ;;[0.15 0.15 0.15 0.5] Aim at Player
  (Transformation|SetActorRotation (Math|Interpolation|RInterpTo (Transformation|GetActorRotation) (Math|Rotator|FindLookatRotation (Transformation|GetActorLocation) (Transformation|GetActorLocation (Game|GetPlayerCharacter 0))) 0.01 15.0)))

(event Custom|Move%20Choice
  ;[0.15 0.15 0.15 0.5] Core Movement
  ;;[0.15 0.15 0.15 0.5] Choice Branching
  (bind _still_in_range (CallFunction|PlayerinRange?))
  (if _still_in_range
    (CallFunction|StayPut)
    (Utilities|FlowControl|DoOnce false :!label _label)
    (elif (Variables|Default|GetReached%20Movement%20Point)
      (CallFunction|BeginChase (Variables|/Game/Assets/Scripts/Player/PlayerBP.PlayerBP_C|GetSpotLight1 (Variables|Default|GetAs%20Player%20BP)))
      (goto _label Reset)
      (else
        (CallFunction|BeginChase (Variables|/Script/Engine.Actor|GetRootComponent (Variables|Default|GetMovement%20Point)))
        (goto _label Reset)))))

(event Custom|Defeat
  (bind _self self)
  (bind _returnvalue (Game|SpawnActorfromClass "/Game/Assets/Enemies/Flying/BP_EnemyDead.BP_EnemyDead_C" (Transformation|GetActorTransform _self) "Undefined" "MultiplyWithRoot" 0 0))
  (Default|DeathSpawn _returnvalue false)
  (Actor|DestroyActor _self))

(event Custom|Check%20Relocation
  ;[0.15 0.15 0.15 0.5] Relocate Functions
  ;;[0.15 0.15 0.15 0.5] Relocation
  (if (>= (Variables|Default|GetShot#) 2)
    (Variables|Default|SetShot# 0)
    (Variables|Default|SetReached%20Movement%20Point false)))

(event EventBeginPlay
  ;[0.15 0.15 0.15 0.5] Startup
  (bind _asplayer_bp (Utilities|Casting|CastToPlayerBP (Game|GetPlayerCharacter 0)))
  (Variables|Default|SetAs%20Player%20BP _asplayer_bp)
  (Variables|Default|SetAccel/Tunring (Math|Random|RandomFloatinRange 1.2e+03 1.4e+03))
  (CallFunction|SpawnTargetLocation)
  (CallFunction|BeginChase (Variables|/Script/Engine.Actor|GetRootComponent (Variables|Default|GetMovement%20Point)))
  (Utilities|Time|SetTimerbyFunctionName 0 "Look!" 0.01 true)
  (Utilities|Time|SetTimerbyFunctionName 0 "Move Choice" 0.1 true true))

(event Collision|EventActorBeginOverlap
  (params (OtherActor :type Actor%20Object%20Reference)))

(event EventTick
  (params (DeltaSeconds :type Float%20%28single-precision%29)))

(event Game|Damage|EventAnyDamage
  (params (Damage :type Float%20%28single-precision%29) (DamageType :type Damage%20Type%20Object%20Reference) (InstigatedBy :type Controller%20Object%20Reference) (DamageCauser :type Actor%20Object%20Reference))
  (bind _output_get (Variables|Default|SetHP 0.0))
  (if (<= _output_get 0.0)
    (CallFunction|Defeat)))

(fn ConstructionScript)

(fn PlayerinRange?
  (bind _ideal_range (Variables|Default|GetIdeal%20Range))
  (bind (_hitlocation _hitnormal _bonename _outhit _returnvalue) (Class|PrimitiveComponent|SphereOverlapComponent (Variables|/Script/Engine.Character|GetCapsuleComponent (Variables|Default|GetAs%20Player%20BP)) (Transformation|GetWorldLocation _ideal_range) (Components|Sphere|GetScaledSphereRadius _ideal_range) false false false))
  (return _returnvalue _hitlocation))